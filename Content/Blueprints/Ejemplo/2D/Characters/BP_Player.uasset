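; BP_Player is a 2D player character that moves along the world X axis and jumps.
; BeginPlay registers the IMC_Personaje_Inputs Enhanced Input mapping context with the local player.
; IA_Movimiento feeds movement input, then uses the sign of X acceleration to flip control rotation between zero and 180 degrees of roll.
; IA_Saltar triggers the jump when started.
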(event Input|EnhancedActionEvents|EnhancedInputActionIA_Movimiento
  (params (ActionValue :type Float%20%28double-precision%29) (ElapsedSeconds :type Float%20%28double-precision%29) (TriggeredSeconds :type Float%20%28double-precision%29) (InputAction :type Input%20Action%20Object%20Reference :default "/Game/Blueprints/Inputs/Acciones/IA_Movimiento.IA_Movimiento"))
  (Pawn|Input|AddMovementInput "1.000000,0.000000,0.000000" ActionValue false)
  (Math|Float|CompareFloat (.x (Pawn|Components|CharacterMovement|GetCurrentAcceleration (Variables|Character|GetCharacterMovement))) 0.0
    (:>
      (Pawn|SetControlRotation (Pawn|GetController) (Math|Rotator|MakeRotator 0.0 0.0 0.0)))
    (:<
      (Pawn|SetControlRotation (Pawn|GetController) (Math|Rotator|MakeRotator 1.8e+02 0.0 0.0)))))

(event Input|EnhancedActionEvents|EnhancedInputActionIA_Saltar
  (params (ActionValue :type Boolean) (ElapsedSeconds :type Float%20%28double-precision%29) (TriggeredSeconds :type Float%20%28double-precision%29) (InputAction :type Input%20Action%20Object%20Reference :default "/Game/Blueprints/Inputs/Acciones/IA_Saltar.IA_Saltar"))
  (:Started
    (Character|Jump)))

(event EventBeginPlay
  (bind _asplayer_controller (Utilities|Casting|CastToPlayerController (Pawn|GetController)))
  (Input|AddMappingContext (PlayerController|LocalPlayerSubsystems|GetEnhancedInputLocalPlayerSubsystem _asplayer_controller) "/Game/Blueprints/Inputs/IMC_Personaje_Inputs.IMC_Personaje_Inputs" 0 "(bIgnoreAllPressedKeysUntilRelease=True,bForceImmediately=False,bNotifyUserSettings=False)"))

(fn ConstructionScript)