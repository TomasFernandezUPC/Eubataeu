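; Player character for a 2D side-scroller, with Enhanced Input movement along X, jumping, shooting, reloading and quitting.
; Movement flips control yaw to face the travel direction, and firing spawns Bala_Player after a delay while ammo remains.
; External events add coins, apply damage or start a timer-counted special-gun power-up that later resets stats.
; Lethal damage or the Vacio event destroys the pawn and shows the Respaw widget; Tick prints health and ammo.
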(event Custom|Special_Power
  (if (Variables|Default|GetSpecial_Pow_Loop)
    (if (== (Variables|Default|GetSpecial_Pow) 6.0)
      (Variables|Default|SetSpecial_Pow 0.0)
      (Variables|Default|SetVelocidad 1.0)
      (Variables|Default|SetVida 1e+02)
      (Variables|Default|SetBalas 6)
      (Variables|Default|SetVelocidad_Dispar 0.4)
      (Variables|Default|SetSpecial_Pow_Loop false)
      (else
        (Variables|Default|SetSpecial_Pow (+ 1.0 (Variables|Default|GetSpecial_Pow)))
        (Variables|Default|SetVelocidad (stale EventSpGun Velocidad))
        (Variables|Default|SetBalas (stale EventSpGun Balas))
        (Variables|Default|SetVida (stale EventSpGun Life))
        (Variables|Default|SetVelocidad_Dispar (stale EventSpGun Velocidad_Disparo))
        (Variables|Default|SetSpecial_Pow_Loop true)))))

(event Input|EnhancedActionEvents|EnhancedInputActionIA_Salir
  (params (ActionValue :type Boolean) (ElapsedSeconds :type Float%20%28double-precision%29) (TriggeredSeconds :type Float%20%28double-precision%29) (InputAction :type Input%20Action%20Object%20Reference :default "/Game/Blueprints/Inputs/Acciones/IA_Salir.IA_Salir"))
  (Game|QuitGame 0 "Quit" false))

(event Input|EnhancedActionEvents|EnhancedInputActionIA_Saltar
  (params (ActionValue :type Boolean) (ElapsedSeconds :type Float%20%28double-precision%29) (TriggeredSeconds :type Float%20%28double-precision%29) (InputAction :type Input%20Action%20Object%20Reference :default "/Game/Blueprints/Inputs/Acciones/IA_Saltar.IA_Saltar"))
  (:Started
    (Character|Jump)))

(event Input|EnhancedActionEvents|EnhancedInputActionIA_Disparar
  (params (ActionValue :type Boolean) (ElapsedSeconds :type Float%20%28double-precision%29) (TriggeredSeconds :type Float%20%28double-precision%29) (InputAction :type Input%20Action%20Object%20Reference :default "/Game/Blueprints/Inputs/Acciones/IA_Disparar.IA_Disparar"))
  (:Started
    (Variables|Default|SetDispara true)
    (Utilities|FlowControl|Delay (Variables|Default|GetVelocidad_Dispar))
    (if (<= (Variables|Default|GetBalas) 0)
      (Variables|Default|SetDispara false)
      (else
        (Game|SpawnActorfromClass "/Game/2D/Characters/Bala/Bala_Player.Bala_Player_C" (Math|Transform|MakeTransform (+ (Transformation|GetActorLocation) "0.000000,0.000000,-10.000000") "0, 0, 0" "1.000000,1.000000,1.000000") "Undefined" "MultiplyWithRoot" 0 0)
        (Variables|Default|SetDispara false)
        (Variables|Default|SetBalas (- (Variables|Default|GetBalas) 1))))))

(event Input|EnhancedActionEvents|EnhancedInputActionIA_Recargar
  (params (ActionValue :type Boolean) (ElapsedSeconds :type Float%20%28double-precision%29) (TriggeredSeconds :type Float%20%28double-precision%29) (InputAction :type Input%20Action%20Object%20Reference :default "/Game/Blueprints/Inputs/Acciones/IA_Recargar.IA_Recargar"))
  (Variables|Default|SetBalas 6))

(event Input|EnhancedActionEvents|EnhancedInputActionIA_Movimiento
  (params (ActionValue :type Float%20%28double-precision%29) (ElapsedSeconds :type Float%20%28double-precision%29) (TriggeredSeconds :type Float%20%28double-precision%29) (InputAction :type Input%20Action%20Object%20Reference :default "/Game/Blueprints/Inputs/Acciones/IA_Movimiento.IA_Movimiento"))
  (Pawn|Input|AddMovementInput "1.000000,0.000000,0.000000" (* ActionValue (Variables|Default|GetVelocidad)) false)
  (Math|Float|CompareFloat (.x (Pawn|Components|CharacterMovement|GetCurrentAcceleration (Variables|Character|GetCharacterMovement))) 0.0
    (:>
      (Pawn|SetControlRotation (Pawn|GetController) (Math|Rotator|MakeRotator 0.0 0.0 0.0)))
    (:<
      (Pawn|SetControlRotation (Pawn|GetController) (Math|Rotator|MakeRotator 0.0 0.0 1.8e+02)))))

(event EventBeginPlay
  (bind _asplayer_controller (Utilities|Casting|CastToPlayerController (Pawn|GetController)))
  (Input|AddMappingContext (PlayerController|LocalPlayerSubsystems|GetEnhancedInputLocalPlayerSubsystem _asplayer_controller) "/Game/Blueprints/Inputs/IMC_Personaje_Inputs.IMC_Personaje_Inputs" 0 "(bIgnoreAllPressedKeysUntilRelease=True,bForceImmediately=False,bNotifyUserSettings=False)"))

(event EventOBMoneda
  (params (Coins :type Integer))
  (Variables|Default|SetMonedas (+ Coins (Variables|Default|GetMonedas))))

(event EventSpGun
  (params (Life :type Float%20%28double-precision%29) (Balas :type Integer) (Velocidad :type Float%20%28double-precision%29) (Velocidad_Disparo :type Float%20%28double-precision%29))
  (Development|PrintString (Utilities|String|ToString(Boolean) (Variables|Default|GetSpecial_Pow_Loop)))
  (Variables|Default|SetSpecial_Pow_Loop true)
  (Utilities|Time|SetTimerbyEvent (delegate Custom|Special_Power) 1.0 (Variables|Default|GetSpecial_Pow_Loop)))

(event EventDaño
  (params (Daño :type Float%20%28double-precision%29))
  (bind _returnvalue (Game|GetPlayerController 0))
  (bind _output_get (Variables|Default|SetVida (- (Variables|Default|GetVida) Daño)))
  (if (<= _output_get 0.0)
    (Variables|Default|SetMurio true)
    (Utilities|FlowControl|Delay 0.2)
    (Actor|DestroyActor)
    (bind _returnvalue_2 (UserInterface|CreateWidget "/Game/Menu/Respaw.Respaw_C"))
    (UserInterface|Viewport|AddtoViewport _returnvalue_2 0)
    (Variables|/Script/Engine.PlayerController|SetbShowMouseCursor _returnvalue true)
    (Input|SetInputModeGameandUI _returnvalue 0 "DoNotLock" true false)))

(event EventVacio
  (params (Vida :type Float%20%28double-precision%29))
  (bind _returnvalue (Game|GetPlayerController 0))
  (Actor|DestroyActor)
  (bind _returnvalue_2 (UserInterface|CreateWidget "/Game/Menu/Respaw.Respaw_C"))
  (UserInterface|Viewport|AddtoViewport _returnvalue_2 0)
  (Variables|/Script/Engine.PlayerController|SetbShowMouseCursor _returnvalue true)
  (Input|SetInputModeGameandUI _returnvalue 0 "DoNotLock" true false))

(event EventTick
  (params (DeltaSeconds :type Float%20%28single-precision%29))
  (Development|PrintString (Utilities|String|Append "VIDA" (Utilities|String|ToString(Float) (Variables|Default|GetVida))) true true "(R=0.088587,G=1.000000,B=0.000000,A=1.000000)")
  (Development|PrintString (Utilities|String|Append "BALAS" (Utilities|String|ToString(Integer) (Variables|Default|GetBalas))) true true "(R=0.000000,G=0.161832,B=1.000000,A=1.000000)"))

(fn ConstructionScript)