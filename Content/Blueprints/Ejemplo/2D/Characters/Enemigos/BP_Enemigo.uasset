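; BP_Enemigo is a 2D-example enemy that fires bullets automatically and can be destroyed by damage.
; A looping timer started on BeginPlay calls Disparar, which spawns Bala_Enemi at the enemy's location and decrements Balas.
; When Balas runs out, Disparar waits through a short Delay, then refills the magazine.
; The DañoEnemigo event subtracts from Vida and destroys the actor once it reaches zero or below.
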(event Custom|Disparar
  (if (<= (Variables|Default|GetBalas) 0)
    (Utilities|FlowControl|Delay 2.0)
    (Variables|Default|SetBalas 6)
    (else
      (Game|SpawnActorfromClass "/Game/2D/Characters/Bala/Bala_Enemi.Bala_Enemi_C" (Math|Transform|MakeTransform (Transformation|GetActorLocation) "0, 0, 0" "1.000000,1.000000,1.000000") "Undefined" "MultiplyWithRoot" 0 0)
      (Variables|Default|SetBalas (- (Variables|Default|GetBalas) 1)))))

(event EventBeginPlay
  (Utilities|Time|SetTimerbyEvent (delegate Custom|Disparar) 1.0 true))

(event EventDañoEnemigo
  (params (Vida :type Float%20%28double-precision%29))
  (bind _output_get (Variables|Default|SetVida (- (Variables|Default|GetVida) Vida)))
  (if (<= _output_get 0.0)
    (Actor|DestroyActor)))

(fn ConstructionScript)