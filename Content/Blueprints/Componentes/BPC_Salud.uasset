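; BPC_Salud is a health component that tracks current and maximum life and handles damage.
; DisminuirVIda subtracts the damage from VidaActual, clamping the result to a normalized 0–1 range rather than to VIdaMaxima.
; It then fires DisminucionDeVida with current and maximum life and prints both values as debug text.
; BeginPlay and Tick are unused.
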(event EventBeginPlay)

(event EventTick
  (params (DeltaSeconds :type Float%20%28single-precision%29)))

(fn DisminuirVIda
  (params (Daño :type Float%20%28double-precision%29))
  (bind _vida_maxima (Variables|Predeterminado|GetVIda_Maxima))
  (Variables|VIDA|SetVida_Actual (Math|Float|Clamp(Float) (- (Variables|VIDA|GetVida_Actual) Daño)))
  (Default|CallDisminucionDeVida (Variables|VIDA|GetVida_Actual) _vida_maxima)
  (Development|PrintText (Utilities|Text|ToText(Float) (Variables|VIDA|GetVida_Actual) "HalfToEven"))
  (Development|PrintText (Utilities|Text|ToText(Float) _vida_maxima "HalfToEven")))