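; Player Blueprint that handles movement input and tracks current and maximum health.
; On BeginPlay it adds the IMC_Alma Enhanced Input context, and IA_Movimiento moves it along fixed world X and Y axes.
; The BPCLIFE component sets starting health through its Life function, and its EventDismiVida dispatcher triggers damage subtraction from VidaActual.
; Tick prints both health values every frame as debug output.
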(event Custom|Actualizador_De_Vida
  (params (Daño :type Float%20%28double-precision%29))
  (Variables|Default|SetVida_Actual (- (Variables|Default|GetVida_Actual) Daño)))

(event Input|EnhancedActionEvents|EnhancedInputActionIA_Movimiento
  (params (ActionValue :type Vector%202D%20Structure) (ElapsedSeconds :type Float%20%28double-precision%29) (TriggeredSeconds :type Float%20%28double-precision%29) (InputAction :type Input%20Action%20Object%20Reference :default "/Game/Inputs/IA_Movimiento.IA_Movimiento"))
  (bind (_x _y) (Math|Vector2D|BreakVector2D ActionValue))
  ;[0.15 0.15 0.15 0.5] MOVIMIENTO DEL PLAYER
  (Pawn|Input|AddMovementInput "1.000000,0.000000,0.000000" _x false)
  (Pawn|Input|AddMovementInput "0.000000,1.000000,0.000000" _y false))

(event EventBeginPlay
  (|CallParentFunction)
  (bind _asplayer_controller (Utilities|Casting|CastToPlayerController (Pawn|GetController)))
  (Input|AddMappingContext (PlayerController|LocalPlayerSubsystems|GetEnhancedInputLocalPlayerSubsystem _asplayer_controller) "/Game/Inputs/IMC_Alma.IMC_Alma" 0 "(bIgnoreAllPressedKeysUntilRelease=True,bForceImmediately=False,bNotifyUserSettings=False)")
  (bind _vida_inicial (Default|Life (Variables|Default|GetBPC_LIFE) (Variables|Default|GetVida_Actual) (Variables|Default|GetVida_Maxima)))
  (Variables|Default|SetVida_Actual _vida_inicial)
  (EventDispatchers|BindEventtoEventDismiVida (Variables|Default|GetBPC_LIFE) (delegate Custom|Actualizador_De_Vida)))

(event EventTick
  (params (DeltaSeconds :type Float%20%28single-precision%29))
  (Development|PrintString (Utilities|String|ToString(Float) (Variables|Default|GetVida_Actual)))
  (Development|PrintString (Utilities|String|ToString(Float) (Variables|Default|GetVida_Maxima))))

(fn ConstructionScript
  (|CallParentFunction))